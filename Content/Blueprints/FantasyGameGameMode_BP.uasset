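; Game mode Blueprint that creates the HUD on BeginPlay and decides whether to launch the start menu.
; It reads a first-time flag on FantasyGameInstance to tell a first launch from later ones.
; On the first launch it clears the flag, adds the HUD, then calls PauseFunction on the first player character found to open the menu.
; Otherwise it only adds the HUD.
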(event `self.ReceiveBeginPlay`
  ;[1 1 1] Check whether to launch start menu or not
  (bind _asfantasy_game_instance (cast `FantasyGameInstance` (`GameplayStatics.GetGameInstance`)))
  (if (`FantasyGameInstance.IsFirstTimeMenuCalled` _asfantasy_game_instance)
    ;[1 1 1] Make so this will not be called again
    (bind _asfantasy_game_instance_2 (cast `FantasyGameInstance` (`GameplayStatics.GetGameInstance`)))
    (set `FantasyGameInstance.IsFirstTimeMenuCalled` false _asfantasy_game_instance_2)
    ;[1 1 1] Create HUD
    (bind _returnvalue (`|CreateWidget` "/Game/UI/HUD_Widget.HUD_Widget_C"))
    (bind _output_get (set `self.HUD_Reference` _returnvalue))
    (`UserWidget.AddToViewport` _output_get 0)
    ;[1 1 1] Call menu
    (bind _outactors (`GameplayStatics.GetAllActorsOfClass` "/Game/Blueprints/FantasyGameCharacter_BP.FantasyGameCharacter_BP_C"))
    (`/Game/Blueprints/FantasyGameCharacter_BP.PauseFunction` (`KismetArrayLibrary.Array_Get` _outactors))
    (else
      ;[1 1 1] Create HUD
      (bind _returnvalue_2 (`|CreateWidget` "/Game/UI/HUD_Widget.HUD_Widget_C"))
      (bind _output_get_2 (set `self.HUD_Reference` _returnvalue_2))
      (`UserWidget.AddToViewport` _output_get_2 0))))

(fn `UserConstructionScript`)