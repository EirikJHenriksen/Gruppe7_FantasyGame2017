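; Level 1 door that opens by destroying itself once the player can pay its pickup price.
; Each tick it checks whether the FantasyGameCharacter_BP player holds at least DoorPrice in CollectionPickup and stands within a fixed radius of the door.
; When both conditions hold, it subtracts DoorPrice from the player's count and removes the actor, with no interaction input needed.
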(event `self.ReceiveTick`
  (params (DeltaSeconds :type "Float (single-precision)"))
  ;[1 1 1] Check if you have enough pickups for the door
  (bind _asfantasy_game_character_bp (cast `/Game/Blueprints/FantasyGameCharacter_BP` (`GameplayStatics.GetPlayerCharacter` 0)))
  (if (>= (`Gruppe7_FantasyGameCharacter.CollectionPickup` _asfantasy_game_character_bp) (`self.DoorPrice`))
    ;[1 1 1] Then check if you are close enough to door
    (bind _asfantasy_game_character_bp_2 (cast `/Game/Blueprints/FantasyGameCharacter_BP` (`GameplayStatics.GetPlayerCharacter` 0)))
    ;[1 1 1] Remove pickups for opening door
    (if (> 350.0 (`KismetMathLibrary.VSize` (- (`self.K2_GetActorLocation`) (`self.K2_GetActorLocation` _asfantasy_game_character_bp_2))))
      (bind _asfantasy_game_character_bp_3 (cast `/Game/Blueprints/FantasyGameCharacter_BP` (`GameplayStatics.GetPlayerCharacter` 0)))
      (set `Gruppe7_FantasyGameCharacter.CollectionPickup` (- (`Gruppe7_FantasyGameCharacter.CollectionPickup` _asfantasy_game_character_bp_3) (`self.DoorPrice`)) _asfantasy_game_character_bp_3)
      (`self.K2_DestroyActor`))))

(fn `UserConstructionScript`)