(event `self.ReceiveBeginPlay`
  ;[1 1 1] Changes material to fit element type
)

(event `self.ReceiveTick`
  (params (DeltaSeconds :type "Float (single-precision)"))
  (bind (_outhit _returnvalue) (`KismetSystemLibrary.LineTraceSingle` (`self.K2_GetActorLocation`) (`self.K2_GetActorLocation` (`GameplayStatics.GetPlayerCharacter` 0)) "TraceTypeQuery1"))
  (if _returnvalue
    (`KismetSystemLibrary.PrintString` "don't see you")
    (else
      (`KismetSystemLibrary.PrintString` "SEE YOU"))))

(fn `UserConstructionScript`)